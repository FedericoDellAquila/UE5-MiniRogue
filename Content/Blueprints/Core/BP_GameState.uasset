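; Game state Blueprint that times the game session and broadcasts time tick, start, pause, resume and stop events with the elapsed timespan.
; Its SetGameSessionState override starts, resumes, pauses or stops the TimeTracker to match the new state, then calls the parent.
; The tracker runs before the parent call, so the current state still distinguishes a fresh start from WaitingToStart from a resume.
; BeginPlay binds the tracker's delegates, which relay to the game state's own delegates.
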(event `self.ReceiveBeginPlay`
  (bind _timetracker (`self.TimeTracker`))
  (add `TimeTracker.OnTimeTrackerIntervalDelegate` _timetracker (delegate `OnTimeTrackerIntervalDelegate_Event`))
  (add `TimeTracker.OnTimeTrackerPausedDelegate` _timetracker (delegate `OnTimeTrackerPausedDelegate_Event`))
  (add `TimeTracker.OnTimeTrackerStartedDelegate` _timetracker (delegate `OnTimeTrackerStartedDelegate_Event`))
  (add `TimeTracker.OnTimeTrackerStoppedDelegate` _timetracker (delegate `OnTimeTrackerStoppedDelegate_Event`))
  (add `TimeTracker.OnTimeTrackerResumedDelegate` _timetracker (delegate `OnTimeTrackerResumedDelegate_Event`)))

(event `OnTimeTrackerIntervalDelegate_Event`
  (params (ElapsedTimespan :type "Timespan Structure"))
  (`self.OnTimeTickDelegate` ElapsedTimespan))

(event `OnTimeTrackerPausedDelegate_Event`
  (`self.OnTimePausedDelegate` (`TimeTracker.GetElapsedTimespan` (`self.TimeTracker`))))

(event `OnTimeTrackerStartedDelegate_Event`
  (`self.OnTimeStartedDelegate` (`TimeTracker.GetElapsedTimespan` (`self.TimeTracker`))))

(event `OnTimeTrackerStoppedDelegate_Event`
  (`self.OnTimeStoppedDelegate` (`TimeTracker.GetElapsedTimespan` (`self.TimeTracker`))))

(event `OnTimeTrackerResumedDelegate_Event`
  (`self.OnTimeResumedDelegate` (`TimeTracker.GetElapsedTimespan` (`self.TimeTracker`))))

(fn `SetGameSessionState`
  (params (NewGameSessionState :type "EGameSessionState Enum" :default "WaitingToStart"))
  (bind _timetracker (`self.TimeTracker`))
  (`|ExecutionSequence`
    (:`then_0`
      (switch `EGameSessionState` NewGameSessionState
        (:`InProgress`
          (if (`|EnumEquality` (`self.GetGameSessionState`) "WaitingToStart")
            (`TimeTracker.Start` _timetracker 1.0 0.0)
            (else
              (`TimeTracker.Resume` _timetracker))))
        (:`Paused`
          (`TimeTracker.Pause` (`self.TimeTracker`)))
        (:`Finished`
          (`TimeTracker.Stop` (`self.TimeTracker`)))))
    (:`then_1`
      (`parent.SetGameSessionState` NewGameSessionState))))

(fn `UserConstructionScript`)