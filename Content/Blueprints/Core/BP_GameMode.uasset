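; Game mode that pre-simulates dice throws in a separate physics world and plays a battle level sequence.
; On init it sets a seed from the "Seed" URL option or a random fallback, then creates the auto-playing sequence.
; After a short BeginPlay delay, SimulationWorldComponent copies "Floor"-tagged actors, spawns four randomly placed dice and simulates them at the physics timestep.
; Simulation and sequence-finished callbacks only print debug output.
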(event `self.ReceiveBeginPlay`
  (bind _simulationworldcomponent (`self.SimulationWorldComponent`))
  (`KismetSystemLibrary.Delay` 0.2)
  (bind _returnvalue (`SimulationWorldComponent.CreateSimulationWorld` _simulationworldcomponent))
  (if _returnvalue
    (bind _outactors (`GameplayStatics.GetAllActorsWithTag` "Floor"))
    (`SimulationWorldComponent.CopyStaticActors` _simulationworldcomponent _outactors)
    (`SimulationWorldComponent.SpawnPhysicsActors` _simulationworldcomponent "/Game/Blueprints/BP_Dice.BP_Dice_C" (`self.MakeStartingTransforms` 4))
    (`SimulationWorldComponent.SimulatePhysics` _simulationworldcomponent (delegate `CustomEvent`) 300 (`UtilityFunctionsLibrary.GetPhysicsStepDeltaTime`) true)))

(event `CustomEvent`
  (params (PhysicsSimulation :type "Array of PhysicsSimulationData Structure (by ref)"))
  (for _array_element PhysicsSimulation
    (`KismetSystemLibrary.PrintString` (`KismetStringLibrary.Conv_IntToString` (`KismetArrayLibrary.Array_Length` (`.Steps` (break `PhysicsSimulationData` _array_element)))))))

(event `self.OnInitGame`
  (params (MapName :type String) (Options :type String) (ErrorMessage :type String))
  (`self.AssignSeed` Options)
  (bind (_outactor _returnvalue) (`LevelSequencePlayer.CreateLevelSequencePlayer` "/Game/Assets/Sequencer/BattleSequence.BattleSequence" (make `MovieSceneSequencePlaybackSettings` true)))
  (add `MovieSceneSequencePlayer.OnFinished` _returnvalue (delegate `OnFinished_Event`)))

(event `OnFinished_Event`
  (`KismetSystemLibrary.PrintString` "Hello"))

(fn `AssignSeed`
  (params (Options :type String))
  (locals (L_Value :type Integer))
  (bind _returnvalue (`GameplayStatics.GetIntOption` Options "Seed" -1))
  (if (< _returnvalue 0)
    (bind _returnvalue_2 (`SeededRandomFunctionsLibrary.GenerateRandomSeed`))
    (set `local.L_Value` (`KismetMathLibrary.BreakRandomStream` _returnvalue_2))
    (else
      (set `local.L_Value` _returnvalue)))
  (`self.SetSeed` (`KismetMathLibrary.MakeRandomStream` (`local.L_Value`))))

(fn `MakeStartingTransforms`
  (params (Amount :type Integer))
  (returns (Transforms :type "Array of Transform Structure"))
  (locals (L_Transforms :type "Array of Transform Structure"))
  (for _ (range Amount)
    (`KismetArrayLibrary.Array_Add` (`local.L_Transforms`) (`KismetMathLibrary.MakeTransform` (`KismetMathLibrary.MakeVector` (`KismetMathLibrary.RandomFloatInRange` -100.0 100.0) (`KismetMathLibrary.RandomFloatInRange` -100.0 100.0) 300.0) (`KismetMathLibrary.RandomRotator` true))))
  (return (`local.L_Transforms`)))

(fn `UserConstructionScript`)