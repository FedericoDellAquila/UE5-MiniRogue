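; BP_RollManager produces physical dice rolls that land on predetermined values, which it can pick with seeded random.
; It pre-simulates BP_Die actors in a separate physics world with copied "Walls" actors, seeded start transforms and a downward impulse, drawing debug bounds per step.
; To reproduce a roll, it spawns each die at its simulated final transform, rotates the landed face to the desired value, then replays the recorded motion.
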(fn `DetermineDiceValues`
  (params (NumDice :type Integer))
  (returns (ReturnValue :type "Array of Integer"))
  (locals (L_Result :type "Array of Integer"))
  (for _ (range NumDice)
    (`KismetArrayLibrary.Array_Add` (`local.L_Result`) (`SeededRandomFunctionsLibrary.GetSeededIntegerInRange` null 1 6)))
  (return (`local.L_Result`)))

(fn `MakeStartingTransforms`
  (params (Amount :type Integer))
  (returns (Transforms :type "Array of Transform Structure"))
  (locals (L_Transforms :type "Array of Transform Structure"))
  (for _ (range Amount)
    (`KismetArrayLibrary.Array_Add` (`local.L_Transforms`) (`KismetMathLibrary.MakeTransform` (`KismetMathLibrary.MakeVector` (`SeededRandomFunctionsLibrary.GetSeededFloatInRange` null -100.0 100.0) (`SeededRandomFunctionsLibrary.GetSeededFloatInRange` null -100.0 100.0) 519.0) (`SeededRandomFunctionsLibrary.GetSeededRotator` null))))
  (return (`local.L_Transforms`)))

(fn `ReproduceRollSimulation`
  (params (DiceValues :type "Array of Integer (by ref)"))
  (locals (L_SpawnedDie :type "/Game/Blueprints/BP_Die Object Reference") (L_DieDesiredValue :type Integer))
  (bind _l_spawneddie (`local.L_SpawnedDie`))
  (bind _returnvalue (`self.SimulateRoll` (`KismetArrayLibrary.Array_Length` DiceValues)))
  (for (_array_element _array_index) _returnvalue
    (set `local.L_DieDesiredValue` (`|GetArrayItem` DiceValues _array_index))
    (`|ExecutionSequence`
      (:`then_0`
        (bind ((`Steps` _steps)) (break `PhysicsSimulationData` _array_element))
        (bind _returnvalue_2 (`ActorUtilityFunctionLibrary.UObjectSpawnActor` null "/Game/Blueprints/BP_Die.BP_Die_C" (`|GetArrayItem` _steps (`KismetArrayLibrary.Array_LastIndex` _steps))))
        (set `local.L_SpawnedDie` _returnvalue_2))
      (:`then_1`
        (bind _returnvalue_3 (`Die.GetValue` _l_spawneddie))
        (`Die.RotateFromFaceToFace` _l_spawneddie _returnvalue_3 (`local.L_DieDesiredValue`)))
      (:`then_2`
        (`Die.ReproducePhysicsSimulation` (`local.L_SpawnedDie`) _array_element)))))

(fn `SimulateRoll`
  (params (NumDice :type Integer))
  (returns (ReturnValue :type "Array of PhysicsSimulationData Structure"))
  (bind _returnvalue (`self.GetPhysicsWorldSimulationManager`))
  (bind _returnvalue_2 (`PhysicsWorldSimulationManager.CreateSimulationWorld` (`self.GetPhysicsWorldSimulationManager`)))
  (if _returnvalue_2
    (`|ExecutionSequence`
      (:`then_0`
        (bind _outactors (`GameplayStatics.GetAllActorsWithTag` self "Walls"))
        (`PhysicsWorldSimulationManager.CopyStaticActors` (`self.GetPhysicsWorldSimulationManager`) _outactors))
      (:`then_1`
        (bind _spawnedphysicsactors (`PhysicsWorldSimulationManager.SpawnPhysicsActors` (`self.GetPhysicsWorldSimulationManager`) "/Game/Blueprints/BP_Die.BP_Die_C" (`self.MakeStartingTransforms` NumDice)))
        (for _array_element _spawnedphysicsactors
          (`PrimitiveComponent.AddImpulse` (`Die.MeshComponent` _array_element) (0.0 0.0 -55555.0) "None" false)))
      (:`then_2`
        (bind _returnvalue_3 (`PhysicsWorldSimulationManager.PerformPhysicsSimulation` :`self` _returnvalue :`bAutoDestroySimulationWorld` false))
        (for _array_element_2 _returnvalue_3
          (bind ((`Actor` _actor) (`Steps` _steps)) (break `PhysicsSimulationData` _array_element_2))
          (for _array_element_3 _steps
            (`UtilityFunctionsLibrary.DrawActorTransformedBoundingBox` null _array_element_3 _actor)))
        (`PhysicsWorldSimulationManager.DestroySimulationWorld` _returnvalue)
        (return _returnvalue_3)))))

(fn `UserConstructionScript`)