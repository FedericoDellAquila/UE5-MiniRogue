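; BP_Dice is a six-sided physics die actor that rolls on ExecuteRoll and prints the face it lands on.
; Roll enables physics and applies a random angular impulse to the cube; the upward impulse is disconnected.
; On sleep it unbinds the event and reads the text render whose forward vector points up.
; A zero result calls Roll again without rebinding; otherwise physics stops and the actor expires shortly after.
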(event `self.ReceiveBeginPlay`
  (set `self.CachedFaces` (`|MakeArray` (`self.TextRender_1`) (`self.TextRender_2`) (`self.TextRender_3`) (`self.TextRender_4`) (`self.TextRender_5`) (`self.TextRender_6`))))

(event `ExecuteRoll`
  (if (not (`self.bIsRolling`))
    (add `PrimitiveComponent.OnComponentSleep` (`self.Cube`) (`|CreateDelegate` :!event `OnComponentSleep_Event`))
    (`self.Roll`)))

(fn `GetDiceValue`
  (returns (Value :type Integer))
  (locals (L_Value :type Integer :default 0))
  (for _array_element (`self.CachedFaces`)
    (if (`KismetMathLibrary.NearlyEqual_FloatFloat` (`KismetMathLibrary.Dot_VectorVector` (`SceneComponent.GetForwardVector` _array_element) (`KismetMathLibrary.Vector_Up`)) 1.0 0.01)
      (bind _astext_render_component (cast `TextRenderComponent` _array_element))
      (set `local.L_Value` (`KismetStringLibrary.Conv_StringToInt` (`KismetTextLibrary.Conv_TextToString` (`TextRenderComponent.Text` _astext_render_component))))
      (break)))
  (return (`local.L_Value`)))

(fn `GetRandomUpwardDirection`
  (returns (Direction :type "Vector Structure"))
  (locals (L_Direction :type "Vector Structure"))
  (bind _returnvalue (`KismetMathLibrary.Dot_VectorVector` (stale _output_get) (`KismetMathLibrary.Vector_Up`)))
  (while (or (< _returnvalue 0.5) (> _returnvalue 0.8))
    (bind _output_get (set `local.L_Direction` (`KismetMathLibrary.RandomUnitVector`))))
  (return (`local.L_Direction`)))

(fn `OnComponentSleep_Event`
  (params (SleepingComponent :type "PrimitiveComponent Object Reference") (BoneName :type Name))
  (clear `PrimitiveComponent.OnComponentSleep` SleepingComponent)
  (bind _value (`self.GetDiceValue`))
  (if (== _value 0)
    (`self.Roll`)
    (else
      (bind _output_get (set `self.bIsRolling` false))
      (`PrimitiveComponent.SetSimulatePhysics` SleepingComponent _output_get)
      (`self.SetLifeSpan` 2.0)
      (`KismetSystemLibrary.PrintString` (`KismetStringLibrary.Conv_IntToString` _value) true true (struct :`G` 1.0 :`A` 1.0) 10.0))))

(fn `Roll`
  (bind _output_get (set `self.bIsRolling` true))
  (`PrimitiveComponent.SetSimulatePhysics` (`self.Cube`) _output_get)
  (`PrimitiveComponent.AddAngularImpulseInDegrees` (`self.Cube`) (* (`KismetMathLibrary.RandomUnitVector`) (`self.RotationForce`) 10.0) "None" false))

(fn `UserConstructionScript`)