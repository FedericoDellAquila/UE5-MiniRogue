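; BP_MonsterCard is the card actor representing an enemy in a tiny roguelike dungeon game.
; On BeginPlay it reads the enemy data of the current dungeon level from the TinyRogue game mode and sets its HealthComponent's max and current health.
; Level-based enemies scale health with the current room number, while others use their fixed data value.
; It then hands itself to its WBP_MonsterCard widget and refreshes the visuals.
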(event `self.ReceiveBeginPlay`
  (bind _healthcomponent (`self.HealthComponent`))
  (bind _healthcomponent_2 (`self.HealthComponent`))
  (bind _outgamemode (`UtilityFunctionsLibrary.GetTinyRogueGameMode`)
    (:`True`
      (bind _output_get (set `self.EnemyData` (`.Enemy` (break `LevelEnemies` (`.Enemies` (break `DungeonLevelsDataTableRow` (`TinyRogueGameMode.GetCurrentDungeonLevel` _outgamemode)))))))
      (bind ((`HealthType` _healthtype) (`Health` _health)) (break `EnemyData` _output_get))
      (if (`|EnumEquality` _healthtype "LevelBased")
        (bind _returnvalue (+ (`TinyRogueGameMode.GetCurrentRoom` _outgamemode) 1))
        (`HealthComponent.SetMaxHealth` _healthcomponent _returnvalue)
        (`HealthComponent.SetHealth` _healthcomponent _returnvalue)
        (else
          (`HealthComponent.SetMaxHealth` _healthcomponent_2 _health)
          (`HealthComponent.SetHealth` _healthcomponent_2 _health)))
      (bind _aswbp_monster_card (cast `/Game/Blueprints/Cards/UI/WBP_MonsterCard` (`WidgetComponent.GetWidget` (`self.WidgetComponent`))))
      (set `/Game/Blueprints/Cards/UI/WBP_MonsterCard.Owner` self _aswbp_monster_card)
      (`/Game/Blueprints/Cards/UI/WBP_MonsterCard.UpdateDataVisuals` _aswbp_monster_card))))

(event `TestDamage`)

(fn `UserConstructionScript`)