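; BP_Die is a physical die that starts at a random rotation and prints its rolled value when its mesh physics goes to sleep.
; Debug keys 1 to 6 turn the key's display name into a target value and call RotateFromFaceToFace from the current GetValue result.
; Debug key 0 resets the relative rotation of FacesRootComponent.
; Face reading and rotation logic are defined outside this graph.
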(event Custom|OnComponentSleep_Event
  (params (SleepingComponent :type Primitive%20Component%20Object%20Reference) (BoneName :type Name))
  (bind _returnvalue (Class|Die|GetValue))
  (Development|PrintString (Utilities|String|ToString(Integer) _returnvalue)))

(event Custom|Rotate
  (params (Key :type Key%20Structure%20%28by%20ref%29 :default "None"))
  (bind _returnvalue (Class|Die|GetValue))
  (Class|Die|RotatefromFacetoFace _returnvalue (Math|Conversions|ToInteger(Byte) (Utilities|String|ToString(Text) (Class|KismetInputLibrary|KeyGetDisplayName Key false)))))

(event EventBeginPlay
  (Transformation|SetActorRotation (Math|Random|RandomRotator true))
  (EventDispatchers|AssignOnComponentSleep (Variables|Default|GetMeshComponent) (delegate Custom|OnComponentSleep_Event)))

(event Input|KeyboardEvents|DebugKey1
  (params (Key :type Key%20Structure :default "None") (ActionValue :type Input%20Action%20Value%20Structure))
  (:Released
    (CallFunction|Rotate Key)))

(event Input|KeyboardEvents|DebugKey2
  (params (Key :type Key%20Structure :default "None") (ActionValue :type Input%20Action%20Value%20Structure))
  (:Released
    (CallFunction|Rotate Key)))

(event Input|KeyboardEvents|DebugKey3
  (params (Key :type Key%20Structure :default "None") (ActionValue :type Input%20Action%20Value%20Structure))
  (:Released
    (CallFunction|Rotate Key)))

(event Input|KeyboardEvents|DebugKey4
  (params (Key :type Key%20Structure :default "None") (ActionValue :type Input%20Action%20Value%20Structure))
  (:Released
    (CallFunction|Rotate Key)))

(event Input|KeyboardEvents|DebugKey5
  (params (Key :type Key%20Structure :default "None") (ActionValue :type Input%20Action%20Value%20Structure))
  (:Released
    (CallFunction|Rotate Key)))

(event Input|KeyboardEvents|DebugKey6
  (params (Key :type Key%20Structure :default "None") (ActionValue :type Input%20Action%20Value%20Structure))
  (:Released
    (CallFunction|Rotate Key)))

(event Input|KeyboardEvents|DebugKey0
  (params (Key :type Key%20Structure :default "None") (ActionValue :type Input%20Action%20Value%20Structure))
  (:Released
    (Transformation|SetRelativeRotation (Variables|Default|GetFacesRootComponent) "0, 0, 0" false false)))

(fn ConstructionScript)